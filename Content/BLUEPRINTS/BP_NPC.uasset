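; BP_NPC is an AI pawn that wanders randomly until triggered, then chases the player.
; BeginPlay caches the first-person player character.
; Tick either moves toward that player when Triggered is set, or waits a random short Delay before moving to a random reachable nearby point via AIMoveTo.
; SetTriggered switches it to chasing, and nothing here clears that state.
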(event `self.ReceiveBeginPlay`
  (bind _asbp_first_person_character (cast `/Game/FirstPerson/Blueprints/BP_FirstPersonCharacter` (`GameplayStatics.GetPlayerPawn` 0)))
  (set `self.Player` _asbp_first_person_character))

(event `self.ReceiveTick`
  (params (DeltaSeconds :type "Float (single-precision)"))
  (if (`self.triggered`)
    (`self.Trigger`)
    (else
      (`KismetSystemLibrary.Delay` (`KismetMathLibrary.RandomFloatInRange` 1.0 5.0))
      (`self.Patrol`))))

(event `Trigger`
  (`|AIMoveTo` self (0.0 0.0 0.0) (`self.Player`)))

(event `Patrol`
  (`|AIMoveTo` self (`NavigationSystemV1.K2_GetRandomReachablePointInRadius` (`self.K2_GetActorLocation`) 1000.0 null null) null))

(fn `SetTriggered`
  (set `self.triggered` true))

(fn `UserConstructionScript`)